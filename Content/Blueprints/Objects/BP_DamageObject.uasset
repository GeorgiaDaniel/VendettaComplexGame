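; BP_DamageObject is an object that takes weapon damage and is destroyed when its health runs out.
; Its Damage function subtracts the incoming WeaponDamage from Health, prints the new value, then either prints a dead message and destroys the actor at zero or below, or prints an alive message.
; The event graph and construction script hold no logic, so everything runs only when Damage is called.
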(event EventBeginPlay)

(event Collision|EventActorBeginOverlap
  (params (OtherActor :type Actor%20Object%20Reference)))

(event EventTick
  (params (DeltaSeconds :type Float%20%28single-precision%29)))

(fn ConstructionScript)

(fn Damage
  (params (Weapon%20Damage :type Float%20%28single-precision%29))
  (bind _output_get (Variables|Default|SetHealth (- (Variables|Default|GetHealth) Weapon%20Damage)))
  (Development|PrintString (Utilities|String|ToString(Float) _output_get) true true "(R=0.947917,G=1.000000,B=0.895833,A=1.000000)")
  (if (<= (Variables|Default|GetHealth) 0.0)
    (Development|PrintString "Dead")
    (Actor|DestroyActor)
    (else
      (Development|PrintString "Alive")))
  (return))