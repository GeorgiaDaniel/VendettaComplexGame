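; BP_HurtPlayerVolume is a trigger volume that damages the first-person player character when it overlaps the detection box.
; BeginPlay caches the player reference, and the overlap event sends WeaponDamage through DamageMessage if that player still has health, also printing the value.
; A DoOnce precedes the player check and is never reset, so only the first overlap by any actor is evaluated.
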(event OnComponentBeginOverlap(DetectionBox)
  (params (OverlappedComponent :type Primitive%20Component%20Object%20Reference) (OtherActor :type Actor%20Object%20Reference) (OtherComp :type Primitive%20Component%20Object%20Reference) (OtherBodyIndex :type Integer) (bFromSweep :type Boolean) (SweepResult :type Hit%20Result%20Structure%20%28by%20ref%29))
  (bind _playerreference (Variables|Default|GetPlayerReference))
  (Utilities|FlowControl|DoOnce false
    (:Completed
      (if (== OtherActor _playerreference)
        (if (> (Variables|/Game/FirstPersonBP/Blueprints/FirstPersonCharacter.FirstPersonCharacter_C|GetCurrentHealth _playerreference) 0.0)
          (Development|PrintString (Utilities|String|ToString(Float) (Variables|Default|GetWeapon%20Damage)))
          (Class|BPIDamage|Damage(Message) (Variables|Default|GetPlayerReference) (Variables|Default|GetWeapon%20Damage)))))))

(event EventBeginPlay
  ;[1 1 1] Gets player reference
  (bind _asfirst_person_character (Utilities|Casting|CastToFirstPersonCharacter (Game|GetPlayerCharacter 0)))
  (Variables|Default|SetPlayerReference _asfirst_person_character))

(fn ConstructionScript)