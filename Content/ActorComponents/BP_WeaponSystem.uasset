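; Weapon system actor component that equips and swaps a character's weapons, currently implemented only for Bobby.
; SetupWeapons identifies the character and starts Bobby with the Proto-Pistol.
; Four slot events set Pressed flags that WeaponSwap reads to choose the new weapon and slot, skipping slots already held.
; WeaponAttributeCheck then applies hard-coded damage, reload and fire-rate stats and refills the character's ammo to that weapon's maximum, even on swaps.
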(event Custom|SetupWeapons
  (params (Character :type First%20Person%20Character%20Object%20Reference))
  ;[1 1 1] Sets up the weapons that the player should have through the character check and weapon selection
  (bind _output_get (Variables|Default|SetCharacter Character))
  (bind _actualcharacter (CallFunction|CharacterCheck _output_get))
  (switch Utilities|FlowControl|Switch|SwitchonEN_Characters _actualcharacter
    (:NewEnumerator0
      (Development|PrintString "Character Doesn't exist or isn't Finished" true true "(R=1.000000,G=0.000000,B=0.018362,A=1.000000)" 5.0 :!label _label))
    (:NewEnumerator1
      (goto _label))
    (:NewEnumerator2
      (goto _label))
    (:NewEnumerator3
      (goto _label))
    (:NewEnumerator4
      (bind _output_get_2 (Variables|Default|SetCurrentCharacter _actualcharacter))
      (bind _output_get_3 (Variables|Default|SetWeaponsBobby "NewEnumerator0"))
      (switch Utilities|FlowControl|Switch|SwitchonEN_WeaponsBobby _output_get_3
        (:NewEnumerator0
          (CallFunction|WeaponAttributeCheck _output_get_3 _output_get_2)
          (Development|PrintString "Setup Complete" true true "(R=0.000000,G=0.588542,B=0.030121,A=1.000000)" 5.0))))))

(event Custom|SwapToWeapon
  ;[1 1 1] Swaps weapon to slot 1. Note: Change to a multi-character system later
  (Variables|Default|SetPressed1 true)
  (if (Utilities|Enum|NotEqual(Enum) (Variables|Default|GetWeaponSwapper) "NewEnumerator0") ; Check to see if same weapon is already equipped
    (bind (_newweapon _slot) (CallFunction|WeaponSwap (Variables|Default|GetWeaponsBobby) (Variables|Default|GetCurrentCharacter)))
    (Variables|Default|SetWeaponsBobby _newweapon)
    (Variables|Default|SetWeaponSwapper _slot)
    (Development|PrintString (Utilities|String|EnumtoString (Variables|Default|GetWeaponSwapper)))
    (CallFunction|WeaponAttributeCheck (Variables|Default|GetWeaponsBobby) "NewEnumerator0")
    (Variables|Default|SetPressed1 false)
    (else
      (Development|PrintString "Already Holding")
      (Variables|Default|SetPressed1 false))))

(event Custom|SwapToWeaponFour
  ;[1 1 1] Weapon swap to slot 4
  (Variables|Default|SetPressed4 true)
  (if (Utilities|Enum|NotEqual(Enum) (Variables|Default|GetWeaponSwapper) "NewEnumerator3") ; Check to see if same weapon is already equipped
    (bind (_newweapon _slot) (CallFunction|WeaponSwap (Variables|Default|GetWeaponsBobby) (Variables|Default|GetCurrentCharacter)))
    (Variables|Default|SetWeaponsBobby _newweapon)
    (Variables|Default|SetWeaponSwapper _slot)
    (Development|PrintString (Utilities|String|EnumtoString (Variables|Default|GetWeaponSwapper)))
    (CallFunction|WeaponAttributeCheck (Variables|Default|GetWeaponsBobby) "NewEnumerator0")
    (Variables|Default|SetPressed4 false)
    (else
      (Development|PrintString "Already Holding")
      (Variables|Default|SetPressed4 false))))

(event Custom|SwapToWeaponTwo
  ;[1 1 1] Weapon swap to slot 2
  (Variables|Default|SetPressed2 true)
  (if (Utilities|Enum|NotEqual(Enum) (Variables|Default|GetWeaponSwapper) "NewEnumerator1") ; Check to see if same weapon is already equipped
    (bind (_newweapon _slot) (CallFunction|WeaponSwap (Variables|Default|GetWeaponsBobby) (Variables|Default|GetCurrentCharacter)))
    (Variables|Default|SetWeaponsBobby _newweapon)
    (Variables|Default|SetWeaponSwapper _slot)
    (Development|PrintString (Utilities|String|EnumtoString (Variables|Default|GetWeaponSwapper)))
    (CallFunction|WeaponAttributeCheck (Variables|Default|GetWeaponsBobby) "NewEnumerator0")
    (Variables|Default|SetPressed2 false)
    (else
      (Development|PrintString "Already Holding")
      (Variables|Default|SetPressed2 false))))

(event Custom|SwapToWeaponThree
  ;[1 1 1] Weapon swap to slot 3
  (Variables|Default|SetPressed3 true)
  (if (Utilities|Enum|NotEqual(Enum) (Variables|Default|GetWeaponSwapper) "NewEnumerator2") ; Check to see if same weapon is already equipped
    (bind (_newweapon _slot) (CallFunction|WeaponSwap "NewEnumerator1" (Variables|Default|GetCurrentCharacter)))
    (Variables|Default|SetWeaponsBobby _newweapon)
    (Variables|Default|SetWeaponSwapper _slot)
    (Development|PrintString (Utilities|String|EnumtoString (Variables|Default|GetWeaponSwapper)))
    (CallFunction|WeaponAttributeCheck (Variables|Default|GetWeaponsBobby) "NewEnumerator0")
    (Variables|Default|SetPressed3 false)
    (else
      (Development|PrintString "Already Holding")
      (Variables|Default|SetPressed3 false))))

(event EventBeginPlay)

(event EventTick
  (params (DeltaSeconds :type Float%20%28single-precision%29)))

(fn WeaponSwap
  (params (CurrentWeapon :type EN_WeaponsBobby%20Enum :default "NewEnumerator0") (CharacterChecker :type EN_Characters%20Enum :default "NewEnumerator0"))
  ;[1 1 1] Character checking
  (LocalVariables|SetCurrentWeaponSwap CurrentWeapon)
  (if (Utilities|Enum|Equal(Enum) CharacterChecker "NewEnumerator4")
    (if (Variables|Default|GetPressed1)
      ;[1 1 1] Bobby Weapons
      (switch Utilities|FlowControl|Switch|SwitchonEN_WeaponsBobby (LocalVariables|GetCurrentWeaponSwap)
        (:NewEnumerator1
          _)
        (:NewEnumerator2
          _)
        (:NewEnumerator3
          _))
      (bind _output_get (Variables|Default|SetWeaponSwapper "NewEnumerator0"))
      (bind _output_get_2 (Variables|Default|SetWeaponsBobby "NewEnumerator0"))
      (return _output_get_2 _output_get)
      (elif (Variables|Default|GetPressed2)
        (switch Utilities|FlowControl|Switch|SwitchonEN_WeaponsBobby (LocalVariables|GetCurrentWeaponSwap)
          (:NewEnumerator0
            _)
          (:NewEnumerator2
            _)
          (:NewEnumerator3
            _))
        (bind _output_get_3 (Variables|Default|SetWeaponSwapper "NewEnumerator1"))
        (bind _output_get_4 (Variables|Default|SetWeaponsBobby "NewEnumerator1"))
        (return _output_get_4 _output_get_3)
        (elif (Variables|Default|GetPressed3)
          (switch Utilities|FlowControl|Switch|SwitchonEN_WeaponsBobby (LocalVariables|GetCurrentWeaponSwap)
            (:NewEnumerator0
              _)
            (:NewEnumerator1
              _)
            (:NewEnumerator3
              _))
          (bind _output_get_5 (Variables|Default|SetWeaponSwapper "NewEnumerator2"))
          (bind _output_get_6 (Variables|Default|SetWeaponsBobby "NewEnumerator2"))
          (return _output_get_6 _output_get_5)
          (elif (Variables|Default|GetPressed4)
            (switch Utilities|FlowControl|Switch|SwitchonEN_WeaponsBobby (LocalVariables|GetCurrentWeaponSwap)
              (:NewEnumerator0
                _)
              (:NewEnumerator1
                _)
              (:NewEnumerator2
                _))
            (bind _output_get_7 (Variables|Default|SetWeaponSwapper "NewEnumerator3"))
            (bind _output_get_8 (Variables|Default|SetWeaponsBobby "NewEnumerator3"))
            (return _output_get_8 _output_get_7)))))
    (else
      (Development|PrintString "Not Valid Character"))))

(fn CharacterCheck
  (params (CurrentCharacter :type First%20Person%20Character%20Object%20Reference))
  (switch Utilities|FlowControl|Switch|SwitchonEN_Characters (Variables|/Game/FirstPersonBP/Blueprints/FirstPersonCharacter.FirstPersonCharacter_C|GetCurrentCharacter CurrentCharacter)
    (:NewEnumerator0
      (return "NewEnumerator0"))
    (:NewEnumerator1
      (return "NewEnumerator1"))
    (:NewEnumerator2
      (return "NewEnumerator2"))
    (:NewEnumerator3
      (return "NewEnumerator3"))
    (:NewEnumerator4
      (Development|PrintString "Bobby")
      (return "NewEnumerator4"))))

(fn WeaponAttributeCheck
  (params (Current%20Weapon :type EN_WeaponsBobby%20Enum :default "NewEnumerator0") (Current%20Character :type EN_Characters%20Enum :default "NewEnumerator0"))
  (bind _character (Variables|Default|GetCharacter))
  (bind _character_2 (Variables|Default|GetCharacter))
  (bind _character_3 (Variables|Default|GetCharacter))
  (bind _character_4 (Variables|Default|GetCharacter))
  ;[1 1 1] Bobby Weapon Attributes
  (bind _output_get (LocalVariables|SetWeapon Current%20Weapon))
  (switch Utilities|FlowControl|Switch|SwitchonEN_WeaponsBobby _output_get
    (:NewEnumerator0
      (bind _output_get_2 (Variables|/Game/FirstPersonBP/Blueprints/FirstPersonCharacter.FirstPersonCharacter_C|SetMaxAmmo _character_2 12.0))
      (Variables|/Game/FirstPersonBP/Blueprints/FirstPersonCharacter.FirstPersonCharacter_C|SetCurrentAmmo _character_2 _output_get_2)
      (Variables|Default|SetWeaponDamage 3e+01)
      (Variables|Default|SetReloadTime 3.0)
      (Variables|Default|SetRateOfFire 0.5)
      (return))
    (:NewEnumerator1
      (bind _output_get_3 (Variables|/Game/FirstPersonBP/Blueprints/FirstPersonCharacter.FirstPersonCharacter_C|SetMaxAmmo _character_3 28.0))
      (Variables|/Game/FirstPersonBP/Blueprints/FirstPersonCharacter.FirstPersonCharacter_C|SetCurrentAmmo _character_3 _output_get_3)
      (Variables|Default|SetWeaponDamage 25.0)
      (Variables|Default|SetReloadTime 2.5)
      (Variables|Default|SetRateOfFire 0.2)
      (return))
    (:NewEnumerator2
      (bind _output_get_4 (Variables|/Game/FirstPersonBP/Blueprints/FirstPersonCharacter.FirstPersonCharacter_C|SetMaxAmmo _character_4 999.0))
      (Variables|/Game/FirstPersonBP/Blueprints/FirstPersonCharacter.FirstPersonCharacter_C|SetCurrentAmmo _character_4 _output_get_4)
      (Variables|Default|SetWeaponDamage 5e+01)
      (Variables|Default|SetReloadTime 0.0)
      (Variables|Default|SetRateOfFire 0.4)
      (return))
    (:NewEnumerator3
      (bind _output_get_5 (Variables|/Game/FirstPersonBP/Blueprints/FirstPersonCharacter.FirstPersonCharacter_C|SetMaxAmmo _character 3.0))
      (Variables|/Game/FirstPersonBP/Blueprints/FirstPersonCharacter.FirstPersonCharacter_C|SetCurrentAmmo _character _output_get_5)
      (Variables|Default|SetWeaponDamage 1.5e+02)
      (Variables|Default|SetReloadTime 6.0)
      (Variables|Default|SetRateOfFire 4.0)
      (return))))