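; Actor component that assigns each playable character a Merc ability and handles its activation.
; SetupAbilities maps the character to an ability, then applies that ability's passive charge rate and on-hit charge value.
; Only Bobby's Sudden Combustion is implemented: at full charge it sphere-traces around the character and damages BPI_Damage actors, resetting charge only if the trace hits something.
; The other four activation events are empty placeholders.
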(event Custom|SetupAbilities
  (params (Current%20Character :type EN_Characters%20Enum :default "NewEnumerator0") (Character%20Reference :type First%20Person%20Character%20Object%20Reference))
  ;[0.04417 1 0] Setup
  (Variables|Default|SetCharacterReference Character%20Reference)
  (bind _actualability (CallFunction|CharactertoAbility Current%20Character))
  (CallFunction|AbilityAttributeGiver _actualability)
  (Development|PrintString "Ability Obtained...")
  (Development|PrintString (Utilities|String|EnumtoString _actualability) true true "(R=0.000000,G=1.000000,B=0.434503,A=1.000000)"))

(event Custom|BobbyMercAbilityActivate
  (bind _characterreference (Variables|Default|GetCharacterReference))
  (bind _characterreference_2 (Variables|Default|GetCharacterReference))
  (bind _returnvalue (Transformation|GetActorLocation _characterreference_2))
  ;[0 1 0.07479] Bobby Ability (Complete)
  (if (>= (Variables|/Game/FirstPersonBP/Blueprints/FirstPersonCharacter.FirstPersonCharacter_C|GetCurrentMercCharge _characterreference) (Variables|/Game/FirstPersonBP/Blueprints/FirstPersonCharacter.FirstPersonCharacter_C|GetMaxMercCharge _characterreference))
    (bind _outhits (Collision|MultiSphereTraceByChannel _returnvalue (+ _returnvalue "0, 0,0.100000") (Variables|Default|GetSuddenCombustionRadius) "TraceTypeQuery3" false (Utilities|Array|MakeArray (Variables|Default|GetCharacterReference)) "ForDuration" true "(R=1.000000,G=0.000000,B=0.000000,A=1.000000)" "(R=0.000000,G=1.000000,B=0.000000,A=1.000000)" 2e+01))
    (bind _output_get (Variables|Default|SetTargetsHit _outhits))
    (bind _array_element (Utilities|Array|ForEachLoopwithBreak _output_get)
      (:LoopBody
        (if (Utilities|DoesObjectImplementInterface (.HitActor (Collision|BreakHitResult _array_element)) "/Game/Blueprints/Interfaces/BPI_Damage.BPI_Damage_C")
          (Class|BPIDamage|Damage(Message) (.HitActor (Collision|BreakHitResult _array_element)) (Variables|Default|GetAbilityDamage))
          (Variables|/Game/FirstPersonBP/Blueprints/FirstPersonCharacter.FirstPersonCharacter_C|SetCurrentMercCharge (Variables|Default|GetCharacterReference) 0.0)
          (else
            (Variables|/Game/FirstPersonBP/Blueprints/FirstPersonCharacter.FirstPersonCharacter_C|SetCurrentMercCharge (Variables|Default|GetCharacterReference) 0.0)))))
    (else
      (Development|PrintString "Ability Not Ready!" true true "(R=1.000000,G=0.000000,B=0.027276,A=1.000000)"))))

(event Custom|VincentMercAbilityActivate
  ;[1 1 1] Vincent Ability (Coming Soon)
)

(event Custom|AzarelMercAbilityActivate
  ;[1 1 1] Azarel Ability (Coming Soon)
)

(event Custom|EllieMercAbilityActivate
  ;[1 1 1] Ellie Ability (Coming Soon)
)

(event Custom|SaraMercAbilityActivate
  ;[1 1 1] Sara Ability (Coming Soon)
)

(event EventBeginPlay)

(event EventTick
  (params (DeltaSeconds :type Float%20%28single-precision%29)))

(fn CharactertoAbility
  (params (CurrentCharacter :type EN_Characters%20Enum :default "NewEnumerator0"))
  (switch Utilities|FlowControl|Switch|SwitchonEN_Characters CurrentCharacter
    (:NewEnumerator0
      (bind _output_get (Variables|Default|SetCurrentMercAbility "NewEnumerator0"))
      (return _output_get))
    (:NewEnumerator1
      (bind _output_get_2 (Variables|Default|SetCurrentMercAbility "NewEnumerator2"))
      (return _output_get_2))
    (:NewEnumerator2
      (bind _output_get_3 (Variables|Default|SetCurrentMercAbility "NewEnumerator3"))
      (return _output_get_3))
    (:NewEnumerator3
      (bind _output_get_4 (Variables|Default|SetCurrentMercAbility "NewEnumerator1"))
      (return _output_get_4))
    (:NewEnumerator4
      (bind _output_get_5 (Variables|Default|SetCurrentMercAbility "NewEnumerator4"))
      (return _output_get_5))))

(fn AbilityAttributeGiver
  (params (Current%20Merc%20Ability :type EN_MercAbilities%20Enum :default "NewEnumerator0"))
  (bind _characterreference (Variables|Default|GetCharacterReference))
  (bind _characterreference_2 (Variables|Default|GetCharacterReference))
  (switch Utilities|FlowControl|Switch|SwitchonEN_MercAbilities Current%20Merc%20Ability
    (:NewEnumerator0
      (Variables|/Game/FirstPersonBP/Blueprints/FirstPersonCharacter.FirstPersonCharacter_C|SetPassiveMercCharge _characterreference (Variables|Default|GetPortalSummonPassiveCharge))
      (Variables|Default|SetChargeOnHit (Variables|Default|GetChargeOnHitPortal)))
    (:NewEnumerator1
      (Variables|/Game/FirstPersonBP/Blueprints/FirstPersonCharacter.FirstPersonCharacter_C|SetPassiveMercCharge _characterreference (Variables|Default|GetRapidBeatdownPassiveCharge))
      (Variables|Default|SetChargeOnHit (Variables|Default|GetChargeOnHitRapid)))
    (:NewEnumerator2
      (Variables|/Game/FirstPersonBP/Blueprints/FirstPersonCharacter.FirstPersonCharacter_C|SetPassiveMercCharge _characterreference_2 (Variables|Default|GetTimeStopPassiveCharge))
      (Variables|Default|SetChargeOnHit (Variables|Default|GetChargeOnHitTime)))
    (:NewEnumerator3
      (Variables|/Game/FirstPersonBP/Blueprints/FirstPersonCharacter.FirstPersonCharacter_C|SetPassiveMercCharge _characterreference_2 (Variables|Default|GetWarMachinePassiveCharge))
      (Variables|Default|SetChargeOnHit (Variables|Default|GetChargeOnHitWar)))
    (:NewEnumerator4
      (Variables|/Game/FirstPersonBP/Blueprints/FirstPersonCharacter.FirstPersonCharacter_C|SetPassiveMercCharge (Variables|Default|GetCharacterReference) (Variables|Default|GetSuddenCombustionPassiveCharge))
      (Variables|Default|SetChargeOnHit (Variables|Default|GetChargeOnHitSudden))
      (Variables|Default|SetAbilityDamage (Variables|Default|GetSuddenCombustionDamage))))
  (return))