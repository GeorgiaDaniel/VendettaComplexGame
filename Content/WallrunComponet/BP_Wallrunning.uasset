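; Wallrun component that lets a falling character run along walls and jump off them.
; A looping timer line-traces right, then left; on a valid wall, LaunchCharacter pushes along the normal-cross-up direction while gravity interpolates toward a wallrun value.
; A faster timer rolls the control rotation to tilt the camera by wall side.
; Ending a run restores gravity and briefly suppresses reattachment; jumping launches away along the wall normal.
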(event Custom|Setup
  (params (Character :type Character%20Object%20Reference))
  (bind _output_get (Variables|Default|SetCharacter Character))
  (bind _output_get_2 (Variables|Default|SetCharacter%20Movement (Variables|/Script/Engine.Character|GetCharacterMovement _output_get)))
  (Variables|Default|SetDefaultGravity (Variables|/Script/Engine.CharacterMovementComponent|GetGravityScale _output_get_2))
  (Utilities|Time|SetTimerbyEvent (delegate Custom|WallRunUpdateEvent) 0.1 true)
  (Utilities|Time|SetTimerbyEvent (delegate Custom|CustomEvent_0) 0.01 true))

(event Custom|JumpEvent
  (CallFunction|WallRunJump))

(event Custom|CustomEvent_0
  (CallFunction|CameraTick))

(event Custom|LandEvent
  (CallFunction|EndWallRun 0.0)
  (Variables|Default|SetWallRunSuppresed false))

(event Custom|WallRunUpdateEvent
  (if (not (Variables|Default|GetWallRunSuppresed))
    (CallFunction|WallRunUpdate)))

(event Custom|ResetWallRunSuppression
  (Utilities|Time|ClearTimerbyFunctionName 0 "ResetWallRunSuppression")
  (Variables|Default|SetWallRunSuppresed false)
  (Development|PrintString "Reset"))

(event EventTick
  (params (DeltaSeconds :type Float%20%28single-precision%29)))

(fn WallRunUpdate
  (bind _onwall (CallFunction|WallRunMovement (Transformation|GetActorLocation (Variables|Default|GetCharacter)) (.Right (Utilities|WallRunEndVectors)) -1.0)) ; Right
  (if _onwall
    (bind _output_get (Variables|Default|SetIsWallruning true))
    (Variables|Default|SetIsWallRunningRight _output_get)
    (Variables|Default|SetIsWallRunningLeft false)
    (bind _output_get_2 (Variables|/Script/Engine.CharacterMovementComponent|SetGravityScale (Variables|Default|GetCharacter%20Movement) (Math|Interpolation|FInterpTo (Variables|/Script/Engine.CharacterMovementComponent|GetGravityScale (Variables|Default|GetCharacter%20Movement)) (Variables|Default|GetWallRunTargetGravity) (Utilities|Time|GetWorldDeltaSeconds) 1e+01) :!label _label))
    (Development|PrintString (Utilities|String|ToString(Float) _output_get_2))
    (elif (Variables|Default|GetIsWallRunningRight)
      (CallFunction|EndWallRun 1.0)
      (else
        (bind _onwall_2 (CallFunction|WallRunMovement (Transformation|GetActorLocation (Variables|Default|GetCharacter)) (.Left (Utilities|WallRunEndVectors)) 1.0))
        (if _onwall_2
          (Variables|Default|SetIsWallruning true)
          (Variables|Default|SetIsWallRunningRight false)
          (Variables|Default|SetIsWallRunningLeft true)
          (goto _label)
          (else
            (CallFunction|EndWallRun 1.0)))))))

(fn WallRunMovement
  (params (Start :type Vector) (End :type Vector) (WallRunDirection :type Float%20%28single-precision%29))
  (Variables|Default|SetStoppedWallRunning false)
  (bind _outhit (Collision|LineTraceByChannel Start End "TraceTypeQuery1" false 0 "None"))
  (if (.bblockinghit _outhit)
    (if (and (AI|Components|NavMovement|IsFalling (Variables|Default|GetCharacter%20Movement)) (.ReturnValue (Utilities|ValidWallRunVector (.normal _outhit))))
      (Variables|Default|SetWallRunNormal (.OutputVector (Utilities|ValidWallRunVector (.normal _outhit))))
      (Character|LaunchCharacter (Variables|Default|GetCharacter) (Utilities|PlayertoWallVector) true false) ; Stick Character To Wall
      (Character|LaunchCharacter (Variables|Default|GetCharacter) (* (Math|Vector|CrossProduct (Variables|Default|GetWallRunNormal) "0, 0,1.000000") (* (Variables|Default|GetWall%20Run%20Direction) (Variables|Default|GetWallRunSpeed))) true (not (Variables|Default|GetWallRunGravity))) ; Move Character forward on wall
      (return true)
      (else
        (return false)))
    (else
      (return false))))

(fn EndWallRun
  (params (ResetTime :type Float%20%28single-precision%29))
  (if (Variables|Default|GetIsWallruning)
    (Variables|Default|SetIsWallruning false)
    (Variables|Default|SetIsWallRunningRight false)
    (Variables|Default|SetIsWallRunningLeft false)
    (Variables|/Script/Engine.CharacterMovementComponent|SetGravityScale (Variables|Default|GetCharacter%20Movement) (Variables|Default|GetDefaultGravity))
    (Variables|Default|SetStoppedWallRunning true)
    (CallFunction|SuppressWallRun ResetTime)))

(fn SuppressWallRun
  (params (Delay :type Float%20%28single-precision%29))
  (Variables|Default|SetWallRunSuppresed true)
  (Utilities|Time|SetTimerbyFunctionName 0 "ResetWallRunSuppression" Delay))

(fn CameraTick
  (if (Variables|Default|GetIsWallRunningLeft)
    (CallFunction|CameraTilt 15.0)
    (elif (Variables|Default|GetIsWallRunningRight)
      (CallFunction|CameraTilt -15.0)
      (else
        (CallFunction|CameraTilt 0.0)))))

(fn CameraTilt
  (params (TargetX%20%28Roll%29 :type Float%20%28single-precision%29))
  (bind _character (Variables|Default|GetCharacter))
  (bind _returnvalue (Pawn|GetController _character))
  (bind _returnvalue_2 (Pawn|GetControlRotation _returnvalue :!class /Script/Engine.Controller))
  (bind (_roll _pitch _yaw) (Math|Rotator|BreakRotator _returnvalue_2))
  (Pawn|SetControlRotation (Pawn|GetController (Variables|Default|GetCharacter)) (Math|Interpolation|RInterpTo _returnvalue_2 (Math|Rotator|MakeRotator TargetX%20%28Roll%29 _pitch _yaw) (Utilities|Time|GetWorldDeltaSeconds) 1e+01)))

(fn WallRunJump
  (bind _wallrunnormal (Variables|Default|GetWallRunNormal))
  (bind _wallrunjumpoffforce (Variables|Default|GetWallRunJumpOffForce))
  (if (Variables|Default|GetIsWallruning)
    (Variables|Default|SetStoppedWallRunning true)
    (CallFunction|EndWallRun 0.2)
    (Character|LaunchCharacter (Variables|Default|GetCharacter) (Math|Vector|MakeVector (* _wallrunjumpoffforce (.x _wallrunnormal)) (* (.y _wallrunnormal) _wallrunjumpoffforce) (Variables|Default|GetWallRunJumpHeight)) false true)))